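; NPC_AI_BP is an AI controller for guard NPCs, driving behavior and combat response from perception.
; On BeginPlay it loads the PatrolData blackboard and runs the GuardBehavior tree.
; When perception senses an actor lacking the "Enemy" tag, it writes that actor to EnemyKey and sets the controlled TP_Character aiming and shooting.
; Losing sense of such an actor clears the key and both flags.
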(event OnTargetPerceptionUpdated(AIPerception)
  (params (Actor :type Actor%20Object%20Reference) (Stimulus :type AI%20Stimulus%20Structure))
  (bind _returnvalue (Pawn|GetControlledPawn))
  (bind _enemykey (Variables|Default|GetEnemyKey))
  (bind _blackboardcomp (Variables|Default|GetBlackboardComp))
  (if (not (Actor|ActorHasTag Actor "Enemy"))
    (if (.bSuccessfullySensed (Utilities|Struct|BreakAIStimulus Stimulus))
      (AI|Components|Blackboard|SetValueasObject _blackboardcomp _enemykey Actor)
      (bind _astp_character (Utilities|Casting|CastToTP_Character _returnvalue))
      (Variables|/Game/Dynamic/NPC/Behavior/TP_Character.TP_Character_C|SetAiming _astp_character true)
      (Variables|/Game/Dynamic/NPC/Behavior/TP_Character.TP_Character_C|SetShooting _astp_character true)
      (else
        (AI|Components|Blackboard|ClearValue _blackboardcomp _enemykey)
        (bind _astp_character_2 (Utilities|Casting|CastToTP_Character _returnvalue))
        (Variables|/Game/Dynamic/NPC/Behavior/TP_Character.TP_Character_C|SetAiming _astp_character_2 false)
        (Variables|/Game/Dynamic/NPC/Behavior/TP_Character.TP_Character_C|SetShooting _astp_character_2 false)))))

(event EventBeginPlay
  (bind _blackboardcomponent (Class|AIController|UseBlackboard "/Game/Dynamic/NPC/AI/PatrolData.PatrolData"))
  (AI|RunBehaviorTree "/Game/Dynamic/NPC/AI/GuardBehavior.GuardBehavior")
  (Variables|Default|SetBlackboardComp _blackboardcomponent))

(fn ConstructionScript)