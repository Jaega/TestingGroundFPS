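; Tile_BP is a terrain tile Blueprint with a gate that opens only while the player character is inside its LockingVolume.
; The gate locks on BeginPlay, and overlap events filtered by IsPlayerActor call Unlock on entry and Lock on exit.
; Lock and Unlock toggle the Gate's collision and swap its red or green barrier material.
; GetAttachTransform exposes the Arrow component's world transform as an attach point.
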(event OnComponentBeginOverlap(LockingVolume)
  (params (OverlappedComponent :type Primitive%20Component%20Object%20Reference) (OtherActor :type Actor%20Object%20Reference) (OtherComp :type Primitive%20Component%20Object%20Reference) (OtherBodyIndex :type Integer) (bFromSweep :type Boolean) (SweepResult :type Hit%20Result%20Structure%20%28by%20ref%29))
  (Utilities|IsPlayerActor OtherActor)
  (CallFunction|Unlock))

(event OnComponentEndOverlap(LockingVolume)
  (params (OverlappedComponent :type Primitive%20Component%20Object%20Reference) (OtherActor :type Actor%20Object%20Reference) (OtherComp :type Primitive%20Component%20Object%20Reference) (OtherBodyIndex :type Integer))
  (Utilities|IsPlayerActor OtherActor)
  (CallFunction|Lock))

(event EventBeginPlay
  (CallFunction|Lock))

(fn ConstructionScript)

(fn GetAttachTransform
  (return (Transformation|GetWorldTransform (Variables|Default|GetArrow))))

(fn Lock
  (Collision|SetCollisionEnabled (Variables|Default|GetGate) "QueryAndPhysics")
  (Rendering|Material|SetMaterial (Variables|Default|GetGate) 0 "/Game/Dynamic/Terrain/RedBarrier.RedBarrier"))

(fn Unlock
  (Collision|SetCollisionEnabled (Variables|Default|GetGate) "NoCollision")
  (Rendering|Material|SetMaterial (Variables|Default|GetGate) 0 "/Game/Dynamic/Terrain/GreenBarrier.GreenBarrier"))