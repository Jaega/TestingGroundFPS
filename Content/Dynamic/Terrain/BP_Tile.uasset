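; Terrain tile for the Infinite Reign mode that, on BeginPlay, locks its gate, randomly places props and enemy pawns, and darkens the sky sphere.
; The player entering LockingVolume unlocks the gate; leaving relocks it and reports the tile conquered once.
; Player overlap with DestroyVolume destroys the tile and has the game mode spawn another, with an Arrow exposing the attach transform.
; Score-based enemy scaling and the night-mode check are disconnected.
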(event OnComponentBeginOverlap(DestroyVolume)
  (params (OverlappedComponent :type Primitive%20Component%20Object%20Reference) (OtherActor :type Actor%20Object%20Reference) (OtherComp :type Primitive%20Component%20Object%20Reference) (OtherBodyIndex :type Integer) (bFromSweep :type Boolean) (SweepResult :type Hit%20Result%20Structure%20%28by%20ref%29))
  (Utilities|IsPlayerActor OtherActor)
  (Actor|DestroyActor)
  (bind _asinfinite_reign_game_mode (Utilities|Casting|CastToInfiniteReignGameMode (Game|GetGameMode)))
  (Default|SpawnTile _asinfinite_reign_game_mode))

(event OnComponentBeginOverlap(LockingVolume)
  (params (OverlappedComponent :type Primitive%20Component%20Object%20Reference) (OtherActor :type Actor%20Object%20Reference) (OtherComp :type Primitive%20Component%20Object%20Reference) (OtherBodyIndex :type Integer) (bFromSweep :type Boolean) (SweepResult :type Hit%20Result%20Structure%20%28by%20ref%29))
  (Utilities|IsPlayerActor OtherActor)
  (CallFunction|Unlock))

(event OnComponentEndOverlap(LockingVolume)
  (params (OverlappedComponent :type Primitive%20Component%20Object%20Reference) (OtherActor :type Actor%20Object%20Reference) (OtherComp :type Primitive%20Component%20Object%20Reference) (OtherBodyIndex :type Integer))
  (Utilities|IsPlayerActor OtherActor)
  (Utilities|FlowControl|Sequence
    (:then_0
      (CallFunction|Lock))
    (:then_1
      (CallFunction|ConquerNewTile))))

(event EventBeginPlay
  (CallFunction|Lock)
  (Utilities|FlowControl|Sequence
    (:then_1
      (Class|Tile|PlaceActors "/Game/Dynamic/Terrain/BP_Container.BP_Container_C" (Utilities|Struct|MakeSpawnParameter 2 3 4e+02))
      (Class|Tile|PlaceActors "/Game/Dynamic/Terrain/BP_Box.BP_Box_C" (Utilities|Struct|MakeSpawnParameter 3 5 1e+02))
      (Class|Tile|PlaceActors "/Game/Dynamic/Terrain/BP_Rock05.BP_Rock05_C" (Utilities|Struct|MakeSpawnParameter 1 2 2.5e+02 1.0 4.0))
      (Class|Tile|PlaceActors "/Game/Dynamic/Terrain/BP_Rock17.BP_Rock17_C" (Utilities|Struct|MakeSpawnParameter 1 2 2.5e+02 1.0 4.0))
      (Class|Tile|PlaceActors "/Game/Dynamic/Terrain/BP_Sack.BP_Sack_C" (Utilities|Struct|MakeSpawnParameter 3 5 2.5e+02))
      (Class|Tile|PlaceAIPawns "/Game/Dynamic/Character/Behavior/BP_Character.BP_Character_C" (Utilities|Struct|MakeSpawnParameter (Variables|Default|GetMinEnemies) (Variables|Default|GetMaxEnemies) 1e+02))
      (CallFunction|ChangeSkySphere))))

(fn ConstructionScript)

(fn GetAttachTransform
  (return (Transformation|GetWorldTransform (Variables|Default|GetArrow))))

(fn Lock
  (Collision|SetCollisionEnabled (Variables|Default|GetGate) "QueryAndPhysics")
  (Rendering|Material|SetMaterial (Variables|Default|GetGate) 0 "/Game/Dynamic/Terrain/MI_Barrier_Red.MI_Barrier_Red"))

(fn Unlock
  (Collision|SetCollisionEnabled (Variables|Default|GetGate) "PhysicsOnly")
  (Rendering|Material|SetMaterial (Variables|Default|GetGate) 0 "/Game/Dynamic/Terrain/MI_Barrier_Green.MI_Barrier_Green"))

(fn ConquerNewTile
  (if (not (Variables|Default|GetIsTileConquered))
    (bind _asinfinite_reign_game_mode (Utilities|Casting|CastToInfiniteReignGameMode (Game|GetGameMode)))
    (Default|NewTileConquered _asinfinite_reign_game_mode)
    (Variables|Default|SetIsTileConquered true)))

(fn ChangeSkySphere
  (bind _outactors (Actor|GetAllActorsOfClass "/Engine/EngineSky/BP_Sky_Sphere.BP_Sky_Sphere_C"))
  (Utilities|FlowControl|Sequence
    (:then_0
      (Rendering|Material|SetVectorParameterValue (Variables|/Engine/EngineSky/BP_Sky_Sphere.BP_Sky_Sphere_C|GetSky%20material (Utilities|Array|Get(acopy) _outactors)) "Zenith Color" "(R=0.000000,G=0.004777,B=0.004777,A=1.000000)" :!class /Script/Engine.MaterialInstanceDynamic))
    (:then_1
      (Rendering|Material|SetVectorParameterValue (Variables|/Engine/EngineSky/BP_Sky_Sphere.BP_Sky_Sphere_C|GetSky%20material (Utilities|Array|Get(acopy) _outactors)) "Horizon color" "(R=0.000000,G=0.004777,B=0.004777,A=1.000000)" :!class /Script/Engine.MaterialInstanceDynamic))
    (:then_2
      (Rendering|Material|SetVectorParameterValue (Variables|/Engine/EngineSky/BP_Sky_Sphere.BP_Sky_Sphere_C|GetSky%20material (Utilities|Array|Get(acopy) _outactors)) "Cloud color" "(R=0.008023,G=0.009134,B=0.010330,A=1.000000)" :!class /Script/Engine.MaterialInstanceDynamic))
    (:then_3
      (Rendering|Material|SetVectorParameterValue (Variables|/Engine/EngineSky/BP_Sky_Sphere.BP_Sky_Sphere_C|GetSky%20material (Utilities|Array|Get(acopy) _outactors)) "Overall Color" "(R=0.423268,G=0.973445,B=0.973445,A=1.000000)" :!class /Script/Engine.MaterialInstanceDynamic))))