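; AI controller for guard NPCs that turns perception events into blackboard state for the GuardBehavior tree.
; On BeginPlay it sets up the PatrolData blackboard, runs the tree and caches the blackboard component.
; Perception updates ignore actors tagged "Enemy"; for others, sight stores the actor as the enemy and hearing stores the sound location.
; Any unsuccessful stimulus from those actors clears the enemy key, whatever the sense.
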(event OnTargetPerceptionUpdated(AIPerception)
  (params (Actor :type Actor%20Object%20Reference) (Stimulus :type AI%20Stimulus%20Structure))
  (bind (_age _expirationage _strength _stimuluslocation _receiverlocation _tag _bsuccessfullysensed) (Utilities|Struct|BreakAIStimulus Stimulus))
  (bind _enemykey (Variables|Default|GetEnemyKey))
  (bind _blackboardcomp (Variables|Default|GetBlackboardComp))
  (if (not (Actor|ActorHasTag Actor "Enemy"))
    (if _bsuccessfullysensed
      (bind _returnvalue (Class|AIPerceptionSystem|GetSenseClassforStimulus Stimulus))
      (Utilities|FlowControl|Sequence
        (:then_0
          (if (== _returnvalue "/Script/AIModule.AISense_Sight")
            (AI|Components|Blackboard|SetValueasObject _blackboardcomp _enemykey Actor)))
        (:then_1
          (if (== _returnvalue "/Script/AIModule.AISense_Hearing")
            (AI|Components|Blackboard|SetValueasVector _blackboardcomp (Variables|Default|GetSoundSourceKey) _stimuluslocation))))
      (else
        (AI|Components|Blackboard|ClearValue _blackboardcomp _enemykey)))))

(event EventBeginPlay
  (bind _blackboardcomponent (Class|AIController|UseBlackboard "/Game/Dynamic/Character/AI/PatrolData.PatrolData"))
  (AI|RunBehaviorTree "/Game/Dynamic/Character/AI/GuardBehavior.GuardBehavior")
  (Variables|Default|SetBlackboardComp _blackboardcomponent))

(fn ConstructionScript)